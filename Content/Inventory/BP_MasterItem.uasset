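; BP_MasterItem is a world item actor that adds its item to, or removes it from, an overlapping pawn's inventory.
; Sphere overlap accepts only BP_inventoryPawn and calls its BPInventory component, with the Remove flag choosing between AddItem and RemoveItemByItemInfo.
; On success the actor destroys itself; otherwise it stores the returned balance in Item and stays in the world.
; Debug strings print some outcomes.
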(event `self.Sphere.OnComponentBeginOverlap`
  (params (OverlappedComponent :type "PrimitiveComponent Object Reference") (OtherActor :type "Actor Object Reference") (OtherComp :type "PrimitiveComponent Object Reference") (OtherBodyIndex :type Integer) (bFromSweep :type Boolean) (SweepResult :type "HitResult Structure (by ref)"))
  (bind (_item_amount _item_item) (break `/Game/Inventory/Str/Inventory_str` (`self.Item`)))
  (bind (_amount _item) (break `/Game/Inventory/Str/Inventory_str` (`self.Item`)))
  (bind _asbp_inventory_pawn (cast `/Game/Inventory/BP_inventoryPawn` OtherActor))
  (if (`self.Remove`)
    (bind _bp_inventory (`/Game/Inventory/BP_inventoryPawn.BP_inventory` _asbp_inventory_pawn))
    (bind (_succes _balance) (`/Game/Inventory/BP_inventory.Remove item by item info` _bp_inventory _amount _item))
    (if _succes
      (`KismetSystemLibrary.PrintString` "item will destroy")
      (`self.K2_DestroyActor`)
      (else
        (`KismetSystemLibrary.PrintString` (`KismetStringLibrary.Concat_StrStr` "Balance is:::" (`KismetStringLibrary.Conv_IntToString` _balance)))
        (set `self.Item` (make `/Game/Inventory/Str/Inventory_str` _balance _item_item))))
    (else
      (bind (_succes_2 _balance_2 _balance_amount) (`/Game/Inventory/BP_inventory.Add item` _bp_inventory _item _amount))
      (if _succes_2
        (`KismetSystemLibrary.PrintString` "item will destroy")
        (`self.K2_DestroyActor`)
        (else
          (set `self.Item` (make `/Game/Inventory/Str/Inventory_str` _balance_amount _balance_2)))))))

(fn `UserConstructionScript`)