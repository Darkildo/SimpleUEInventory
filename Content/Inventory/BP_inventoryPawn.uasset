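; Inventory pawn that shows the live state of its BPInventory as on-screen debug text.
; Tick sets its own interval to a tenth of a second, then prints current volume and weight against their maximums, plus the free slot count.
; It also loops through every slot to print index, item name, amount and ID, with print durations matching the tick interval so the readout refreshes in place.
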(event `self.ReceiveTick`
  (params (DeltaSeconds :type "Float (single-precision)"))
  (bind _bp_inventory (`self.BP_inventory`))
  (bind _bp_inventory_2 (`self.BP_inventory`))
  (`self.SetActorTickInterval` 0.1)
  (bind _value (`/Game/Inventory/BPI_inventory.Get inventory Volume` _bp_inventory))
  (`KismetSystemLibrary.PrintString` (`KismetStringLibrary.Concat_StrStr` "Inventory Volume is:" "" (`KismetStringLibrary.Conv_DoubleToString` _value) "/" (`KismetStringLibrary.Conv_DoubleToString` (`/Game/Inventory/BP_inventory.Max Volume` _bp_inventory))) true true (struct :`R` 0.057427 :`G` 0.104014 :`B` 0.380208 :`A` 1.0) 0.1)
  (bind _weight (`/Game/Inventory/BPI_inventory.Get inventory Weight` _bp_inventory_2))
  (`KismetSystemLibrary.PrintString` (`KismetStringLibrary.Concat_StrStr` "Inventory Weight is:" "" (`KismetStringLibrary.Conv_DoubleToString` _weight) "/" (`KismetStringLibrary.Conv_DoubleToString` (`/Game/Inventory/BP_inventory.Max Weight` _bp_inventory_2))) true true (struct :`R` 0.057427 :`G` 0.104014 :`B` 0.380208 :`A` 1.0) 0.1)
  (bind _newparam (`/Game/Inventory/BPI_inventory.Get current amount of free slots` (`self.BP_inventory`)))
  (`KismetSystemLibrary.PrintString` (`KismetStringLibrary.Concat_StrStr` "Amount of free slots in inventory is:" " " (`KismetStringLibrary.Conv_IntToString` _newparam)) true true (struct :`R` 0.057427 :`G` 0.104014 :`B` 0.380208 :`A` 1.0) 0.1)
  (for (_array_element _array_index) (`/Game/Inventory/BP_inventory.Slots` (`self.BP_inventory`))
    (bind (_amount _item) (break `/Game/Inventory/Str/Inventory_str` _array_element))
    (`KismetSystemLibrary.PrintString` (`KismetStringLibrary.Concat_StrStr` (`KismetStringLibrary.Conv_IntToString` _array_index) (`.Name_7_9A4D4F354F9A6994C38324AA08310690` (break `/Game/Inventory/Str/Item_str` _item)) " is:  " (`KismetStringLibrary.Conv_IntToString` _amount) "   " "id: " (`KismetStringLibrary.Conv_IntToString` (break `/Game/Inventory/Str/Item_str` _item))) true true (struct :`R` 0.057427 :`G` 0.104014 :`B` 0.380208 :`A` 1.0) 0.1)))

(fn `UserConstructionScript`)