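; Slot-based inventory that stores items with amounts in an array sized at BeginPlay and provides add, remove, find and capacity queries.
; AddItem tops up matching stacks before using empty slots, recursing one unit at a time when the whole amount does not fit.
; RemoveItem recursively carries shortfalls into other slots holding the same ID.
; Optional custom settings override stack size and cap total volume and weight, both recalculated by scanning the slots.
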(event `self.ReceiveBeginPlay`
  (`self.inventory Construction`))

(event `inventory Construction`
  ;[0.8914 0.1914 1] Some inventory  prepare
  (`|ExecutionSequence`
    (:`then_0`
      ;;[1 0.7462 0.3521] Creating inventory array
      (`KismetArrayLibrary.Array_Resize` (`self.Slots`) (`self.Inventory Slots Amount`)))
    (:`then_1`
      (if (not (`self.Custom Inventory Setting?`))
        (set `self.Use amount?` false)
        (set `self.Use volume?` false)
        (set `self.Use Weight?` false)))))

(fn `Add item`
  (params (Item :type "/Game/Inventory/Str/Item_str Structure") (Amount :type Integer))
  (returns (Succes :type Boolean) (balance :type "/Game/Inventory/Str/Item_str Structure") (`balance Amount` :type Integer))
  (locals (L_item :type "/Game/Inventory/Str/Item_str Structure") (L_amount :type Integer) (L_slot :type Integer :default 0) (L_Stackable :type Boolean :default true) (`L_max stack Size` :type Integer))
  (bind _slots (`self.Slots`))
  (bind _l_slot (`local.L_slot`))
  (bind _l_slot_2 (`local.L_slot`))
  (bind _l_slot_3 (`local.L_slot`))
  (bind _output_amount (break `/Game/Inventory/Str/Inventory_str` (`|GetArrayItem` (`self.Slots`) _l_slot)))
  (bind (_amount _item) (break `/Game/Inventory/Str/Inventory_str` (`|GetArrayItem` (`self.Slots`) _l_slot_2)))
  (if (`self.Inventory is full?`)
    (return false Item (`local.L_amount`))
    (else
      (set `local.L_amount` Amount)
      (bind _output_get (set `local.L_item` Item))
      (bind ((`ID_6_792DAEB048A3F3C884D2A7B0A695BC53` _id) (`Stackable?_19_7285F233478DB3EE1132F59C6BDB9624` _stackable_)) (break `/Game/Inventory/Str/Item_str` _output_get))
      (if _stackable_
        (set `local.L_Stackable` true)
        (bind (_succes _slot) (`self.Find item in inventory by id with free amount` _id))
        (if _succes
          ;[1 1 1] Add more item in the L slot if we already have this item in inventory
          (set `local.L_slot` _slot)
          (if (`self.Can add this amount of item in slot` (`local.L_amount`) _l_slot_2 (`local.L_Stackable`) (`local.L_item`))
            (`KismetArrayLibrary.Array_Set` (`self.Slots`) _l_slot_3 (make `/Game/Inventory/Str/Inventory_str` (+ (`local.L_amount`) _amount) _item))
            (elif (`self.Can add this amount of item in slot` 1 (`local.L_slot`) (`local.L_Stackable`) (`local.L_item`))
              (`KismetArrayLibrary.Array_Set` (`self.Slots`) _l_slot_3 (make `/Game/Inventory/Str/Inventory_str` (+ _amount 1) _item))
              (bind (_succes_2 _balance _balance_amount) (`self.Add item` (`local.L_item`) (- (`local.L_amount`) 1)))
              (return _succes_2 _balance _balance_amount)
              (else
                (return false (`local.L_item`) (`local.L_amount`)))))
          (else
            (bind (_succes_3 _slot_2) (`self.Find free slot in inventory` :!label _label))
            (if _succes_3
              (set `local.L_slot` _slot_2)
              (if (`self.Can add this amount of item in slot` (`local.L_amount`) (`local.L_slot`) (`local.L_Stackable`) (`local.L_item`))
                (`KismetArrayLibrary.Array_Set` _slots (`local.L_slot`) (make `/Game/Inventory/Str/Inventory_str` (+ (`local.L_amount`) (`.Amount_2_AABA3507466E9F1D2CF1D49469CED7D7` (break `/Game/Inventory/Str/Inventory_str` (`|GetArrayItem` _slots (`local.L_slot`))))) (`local.L_item`)))
                (return true (`local.L_item`) 0)
                (elif (`self.Can add this amount of item in slot` 1 (`local.L_slot`) (`local.L_Stackable`) (`local.L_item`))
                  (`KismetArrayLibrary.Array_Set` (`self.Slots`) _l_slot (make `/Game/Inventory/Str/Inventory_str` (+ _output_amount 1) (`local.L_item`)))
                  (bind (_succes_4 _balance_2 _balance_amount_2) (`self.Add item` (`local.L_item`) (- (`local.L_amount`) 1)))
                  (return _succes_4 _balance_2 _balance_amount_2)
                  (else
                    (return false (`local.L_item`) (`local.L_amount`)))))
              (else
                (return false (`local.L_item`) (`local.L_amount`))))))
        (else
          (set `local.L_Stackable` false)
          (goto _label))))))

(fn `Can add this amount of item in slot`
  (params (Amount :type Integer) (Slot :type Integer) (Stackable :type Boolean) (Item :type "/Game/Inventory/Str/Item_str Structure"))
  (returns (Succes :type Boolean))
  (locals (L_amount :type Integer) (L_slot :type Integer))
  (bind _returnvalue (+ (`local.L_amount`) (`.Amount_2_AABA3507466E9F1D2CF1D49469CED7D7` (break `/Game/Inventory/Str/Inventory_str` (`|GetArrayItem` (`self.Slots`) (`local.L_slot`))))))
  (bind _returnvalue_2 (+ (`local.L_amount`) (`.Amount_2_AABA3507466E9F1D2CF1D49469CED7D7` (break `/Game/Inventory/Str/Inventory_str` (`|GetArrayItem` (`self.Slots`) (`local.L_slot`))))))
  (set `local.L_slot` Slot)
  (set `local.L_amount` Amount)
  (if (and (`self.Custom Inventory Setting?`) (`self.Use amount?`))
    ;[1 1 1] Custom items Amount check
    (if (`local.Stackable`)
      (if (> _returnvalue (`self.Max amount Item per slot`))
        (return false)
        (else
          _))
      (elif (== _returnvalue 1)
        _
        (else
          (return false))))
    (else
      ;[0.3458 0.4247 1] Default item amount check
      (if (`local.Stackable`)
        (if (> _returnvalue_2 (`.MaxStackSize_31_0E2304574B17065E311A4BAF717EA7BE` (break `/Game/Inventory/Str/Item_str` (`local.Item`))))
          (return false)
          (else
            _))
        (elif (== _returnvalue_2 1)
          _
          (else
            (return false))))))
  (if (`self.Use volume?`)
    ;[0.2257 0.3841 1] Volume check
    (if (> (+ (`self.Get current volume`) (* (`local.L_amount`) (`.volume_27_B9D6FA734C8BF8DA38976B9A7D108490` (break `/Game/Inventory/Str/Item_str` (`local.Item`))))) (`self.Max Volume`))
      (return false)
      (else
        _)))
  (if (`self.Use Weight?`)
    (if (> (+ (`self.Get current weight`) (* (`local.L_amount`) (`.Weight_24_E4E134DD42133A2ADFE4BC83AAA4B54E` (break `/Game/Inventory/Str/Item_str` (`local.Item`))))) (`self.Max Weight`))
      (return false)
      (else
        (return true)))
    (else
      (return true))))

(fn `Find free slot in inventory`
  (returns (Succes :type Boolean) (Slot :type Integer))
  (for (_array_element _array_index) (`self.Slots`)
    (if (not (!= (`.Amount_2_AABA3507466E9F1D2CF1D49469CED7D7` (break `/Game/Inventory/Str/Inventory_str` _array_element)) 0))
      (return true _array_index)))
  (return false 0))

(fn `Find item in inventory by id`
  (params (Id :type Integer))
  (returns (Succes :type Boolean) (Slot :type Integer))
  (for (_array_element _array_index) (`self.Slots`)
    (bind (_amount _item) (break `/Game/Inventory/Str/Inventory_str` _array_element))
    (if (and (== Id (`.ID_6_792DAEB048A3F3C884D2A7B0A695BC53` (break `/Game/Inventory/Str/Item_str` _item))) (!= _amount 0))
      (return true _array_index)))
  (return false 0))

(fn `Find item in inventory by id with free amount`
  (params (id :type Integer))
  (returns (Succes :type Boolean) (Slot :type Integer))
  (for (_array_element _array_index) (`self.Slots`)
    (if (and (== (`.ID_6_792DAEB048A3F3C884D2A7B0A695BC53` (break `/Game/Inventory/Str/Item_str` (`.item_5_E0B848BC4C001FCC74517699DF1F8361` (break `/Game/Inventory/Str/Inventory_str` _array_element)))) id) (not (`self.Slot is full?` _array_index)))
      (return true _array_index)))
  (return false 0))

(fn `Get Amoutn of free slots`
  (returns (NewParam :type Integer))
  (locals (L_Value :type Integer))
  (for _array_element (`self.Slots`)
    (if (== (`.Amount_2_AABA3507466E9F1D2CF1D49469CED7D7` (break `/Game/Inventory/Str/Inventory_str` _array_element)) 0)
      (`/Engine/EditorBlueprintResources/StandardMacros.IncrementInt` (`local.L_Value`))))
  (return (`local.L_Value`)))

(fn `Get current amount of free slots`
  (returns (NewParam :type Integer))
  (return (`self.Get Amoutn of free slots`)))

(fn `Get current volume`
  (returns (Volume :type "Float (double-precision)"))
  (locals (L_volume :type "Float (double-precision)"))
  (for _array_element (`self.Slots`)
    (bind (_amount _item) (break `/Game/Inventory/Str/Inventory_str` _array_element))
    (if (!= _amount 0)
      (set `local.L_volume` (+ (`local.L_volume`) (* _amount (`.volume_27_B9D6FA734C8BF8DA38976B9A7D108490` (break `/Game/Inventory/Str/Item_str` _item)))))))
  (return (`local.L_volume`)))

(fn `Get current weight`
  (returns (Weight :type "Float (double-precision)"))
  (locals (L_weight :type "Float (double-precision)"))
  (for _array_element (`self.Slots`)
    (bind (_amount _item) (break `/Game/Inventory/Str/Inventory_str` _array_element))
    (if (!= _amount 0)
      (set `local.L_weight` (+ (`local.L_weight`) (* _amount (`.Weight_24_E4E134DD42133A2ADFE4BC83AAA4B54E` (break `/Game/Inventory/Str/Item_str` _item)))))))
  (return (`local.L_weight`)))

(fn `Get inventory Volume`
  (returns (Value :type "Float (double-precision)"))
  (return (`self.Get current volume`)))

(fn `Get inventory Weight`
  (returns (Weight :type "Float (double-precision)"))
  (return (`self.Get current weight`)))

(fn `Inventory is full?`
  (returns (Full :type Boolean))
  (for (_array_element _array_index) (`self.Slots`)
    (if (!= 0 (`.Amount_2_AABA3507466E9F1D2CF1D49469CED7D7` (break `/Game/Inventory/Str/Inventory_str` _array_element)))
      (if (not (`self.Slot is full?` _array_index))
        (if (`self.Custom Inventory Setting?`) :!label _label
          (if (`self.Use volume?`)
            ;[0.4169 0.8177 1] Check Max Volume in inventory
            (if (>= (`self.Get current volume`) (`self.Max Volume`))
              (return true)
              (else
                _)))
          (if (`self.Use Weight?`)
            ;[1 0.9594 0.3846] Check Max Weight in inventory
            (if (>= (`self.Get current weight`) (`self.Max Weight`))
              (return true)
              (else
                (return false)))
            (else
              (return false)))
          (else
            (return false))))
      (else
        (goto _label))))
  (return true))

(fn `Remove item`
  (params (Slot :type Integer) (Value :type Integer))
  (returns (Succes :type Boolean) (Balance :type Integer))
  (locals (L_id :type Integer) (L_res :type Integer :default 0))
  (bind _slots (`self.Slots`))
  (bind _slot (`local.Slot`))
  (bind (_amount _item) (break `/Game/Inventory/Str/Inventory_str` (`|GetArrayItem` _slots (`local.Slot`))))
  (bind _returnvalue (- _amount (`local.Value`)))
  (set `local.L_id` (`.ID_6_792DAEB048A3F3C884D2A7B0A695BC53` (break `/Game/Inventory/Str/Item_str` _item)))
  (if (== _returnvalue 0)
    (`KismetArrayLibrary.Array_Set` _slots (`local.Slot`) (make `/Game/Inventory/Str/Inventory_str` 0))
    (return true 0)
    (else
      (set `local.L_res` (`KismetMathLibrary.Abs_Int` _returnvalue))
      (if (< _returnvalue 0)
        (`KismetArrayLibrary.Array_Set` _slots _slot (make `/Game/Inventory/Str/Inventory_str` 0))
        (bind (_succes _slot_2) (`self.Find item in inventory by id` (`local.L_id`)))
        (if _succes
          (bind _succes_2 (`self.Remove item` _slot_2 (`local.L_res`)))
          (return _succes_2 (`local.L_res`))
          (else
            (return false (`local.L_res`))))
        (else
          (`KismetArrayLibrary.Array_Set` _slots _slot (make `/Game/Inventory/Str/Inventory_str` _returnvalue))
          (return true 0))))))

(fn `Remove item by item info`
  (params (Value :type Integer) (Item :type "/Game/Inventory/Str/Item_str Structure"))
  (returns (Succes :type Boolean) (balance :type Integer))
  (bind (_succes _slot) (`self.Find item in inventory by id` (`.ID_6_792DAEB048A3F3C884D2A7B0A695BC53` (break `/Game/Inventory/Str/Item_str` Item))))
  (if _succes
    (bind (_succes_2 _balance) (`self.Remove item` _slot (`local.Value`)))
    (return _succes_2 _balance)
    (else
      (return false (`local.Value`)))))

(fn `Slot is full?`
  (params (Slot :type Integer))
  (returns (Full :type Boolean))
  (bind (_amount _item) (break `/Game/Inventory/Str/Inventory_str` (`|GetArrayItem` (`self.Slots`) Slot)))
  (bind ((`Stackable?_19_7285F233478DB3EE1132F59C6BDB9624` _stackable_) (`MaxStackSize_31_0E2304574B17065E311A4BAF717EA7BE` _maxstacksize)) (break `/Game/Inventory/Str/Item_str` _item))
  (if _stackable_
    (if (and (`self.Custom Inventory Setting?`) (`self.Use amount?`))
      (return (not (> (`self.Max amount Item per slot`) _amount)))
      (else
        (return (>= _maxstacksize _amount))))
    (else
      (return (>= _amount 1)))))